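; Endless-runner track block that dresses itself with random buildings, sidewalk and road obstacles, and a coin in a free lane.
; Tick slides both road obstacles along -Y as traffic.
; Player overlap asks the game mode for another block and destroys this one after a delay, while obstacle overlaps register hits with immunity and camera shake.
; A front-block truck check is meant to gate car spawning, but its trace result is unwired.
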(event `self.ReceiveTick`
  (params (DeltaSeconds :type "Float (single-precision)"))
  (`self.MoveCars`))

(event `self.ReceiveBeginPlay`
  ;[1 1 1] Spawn Obstacles
  (bind _frontblock (`self.CheckFrontBlock`))
  (`/Engine/EditorBlueprintResources/StandardMacros.IsValid` _frontblock
    (:`Is Valid`
      (set `self.SpawnLane2Car` (not (== (`StaticMeshComponent.StaticMesh` (`/Game/Blueprints/BP_Block.Obstacle2` _frontblock)) "/Game/AssetsvilleTown/Meshes/Vehicles/SM_veh_TruckMerged.SM_veh_TruckMerged")))
      (set `self.SpawnLane2Car` (not (== null (`StaticMeshComponent.StaticMesh` (`/Game/Blueprints/BP_Block.Obstacle3` _frontblock))))))
    (:`Is Not Valid`
      _))
  (`self.Spawn Obstacles`)
  (`self.SpawnCoins`)
  (`self.SpawnBuildings`))

(event `self.OverlapBox.OnComponentBeginOverlap`
  (params (OverlappedComponent :type "PrimitiveComponent Object Reference") (OtherActor :type "Actor Object Reference") (OtherComp :type "PrimitiveComponent Object Reference") (OtherBodyIndex :type Integer) (bFromSweep :type Boolean) (SweepResult :type "HitResult Structure (by ref)"))
  ;[1 1 1] Adding blocks while playing
  (cast `/Game/ThirdPerson/Blueprints/BP_ThirdPersonCharacter` OtherActor)
  (bind _asbp_third_person_game_mode (cast `/Game/ThirdPerson/Blueprints/BP_ThirdPersonGameMode` (`GameplayStatics.GetGameMode`)))
  (`/Game/ThirdPerson/Blueprints/BP_ThirdPersonGameMode.AddBlock` _asbp_third_person_game_mode true)
  (`KismetSystemLibrary.Delay` 5.0)
  (`self.K2_DestroyActor`))

(event `self.Obstacle1.OnComponentBeginOverlap`
  (params (OverlappedComponent :type "PrimitiveComponent Object Reference") (OtherActor :type "Actor Object Reference") (OtherComp :type "PrimitiveComponent Object Reference") (OtherBodyIndex :type Integer) (bFromSweep :type Boolean) (SweepResult :type "HitResult Structure (by ref)"))
  ;[1 1 1] Quit Game on Crash
  (bind _asbp_third_person_character (cast `/Game/ThirdPerson/Blueprints/BP_ThirdPersonCharacter` OtherActor))
  (`self.HitPlayer` _asbp_third_person_character))

(event `self.Obstacle2.OnComponentBeginOverlap`
  (params (OverlappedComponent :type "PrimitiveComponent Object Reference") (OtherActor :type "Actor Object Reference") (OtherComp :type "PrimitiveComponent Object Reference") (OtherBodyIndex :type Integer) (bFromSweep :type Boolean) (SweepResult :type "HitResult Structure (by ref)"))
  ;[1 1 1] Quit Game on Crash
  (bind _asbp_third_person_character (cast `/Game/ThirdPerson/Blueprints/BP_ThirdPersonCharacter` OtherActor))
  (`self.HitPlayer` _asbp_third_person_character))

(event `self.Obstacle3.OnComponentBeginOverlap`
  (params (OverlappedComponent :type "PrimitiveComponent Object Reference") (OtherActor :type "Actor Object Reference") (OtherComp :type "PrimitiveComponent Object Reference") (OtherBodyIndex :type Integer) (bFromSweep :type Boolean) (SweepResult :type "HitResult Structure (by ref)"))
  ;[1 1 1] Quit Game on Crash
  (bind _asbp_third_person_character (cast `/Game/ThirdPerson/Blueprints/BP_ThirdPersonCharacter` OtherActor))
  (`self.HitPlayer` _asbp_third_person_character))

(event `self.Obstacle4.OnComponentBeginOverlap`
  (params (OverlappedComponent :type "PrimitiveComponent Object Reference") (OtherActor :type "Actor Object Reference") (OtherComp :type "PrimitiveComponent Object Reference") (OtherBodyIndex :type Integer) (bFromSweep :type Boolean) (SweepResult :type "HitResult Structure (by ref)"))
  ;[1 1 1] Quit Game on Crash
  (bind _asbp_third_person_character (cast `/Game/ThirdPerson/Blueprints/BP_ThirdPersonCharacter` OtherActor))
  (`self.HitPlayer` _asbp_third_person_character))

(fn `CheckFrontBlock`
  (returns (FrontBlock :type "/Game/Blueprints/BP_Block Object Reference"))
  (bind _returnvalue (`self.K2_GetActorLocation`))
  (bind _outhit (`KismetSystemLibrary.LineTraceSingle` _returnvalue (+ _returnvalue (* (`self.GetActorRightVector`) 2.0)) "TraceTypeQuery1")))

(fn `HitPlayer`
  (params (PlayerRef :type "/Game/ThirdPerson/Blueprints/BP_ThirdPersonCharacter Object Reference"))
  (if (not (`/Game/ThirdPerson/Blueprints/BP_ThirdPersonCharacter.Immune` PlayerRef))
    (`/Game/ThirdPerson/Blueprints/BP_ThirdPersonCharacter.Immunity` PlayerRef)
    (`/Engine/EditorBlueprintResources/StandardMacros.IncrementInt` (`/Game/ThirdPerson/Blueprints/BP_ThirdPersonCharacter.Hits` PlayerRef)
      (:`  `
        (set `/Game/ThirdPerson/Blueprints/BP_ThirdPersonCharacter.SpringArmInterpSpeed` 10.0 PlayerRef)
        (`PlayerController.ClientStartCameraShake` :`self` (`GameplayStatics.GetPlayerController` 0) :`Shake` "/Game/Blueprints/CS_HitObject.CS_HitObject_C")
        (`/Game/ThirdPerson/Blueprints/BP_ThirdPersonCharacter.WaitToRemoveHit` PlayerRef)))))

(fn `MoveCars`
  (bind _obstacle2 (`self.Obstacle2`))
  (bind _obstacle3 (`self.Obstacle3`))
  (`SceneComponent.K2_SetWorldLocation` _obstacle2 (+ (`SceneComponent.K2_GetComponentLocation` _obstacle2) (* (0.0 -1.0 0.0) 10.0)) false false)
  (`SceneComponent.K2_SetWorldLocation` _obstacle3 (+ (`SceneComponent.K2_GetComponentLocation` _obstacle3) (* (0.0 -1.0 0.0) 10.0)) false false))

(fn `Spawn Obstacles`
  (bind _outitem (`KismetArrayLibrary.Array_Random` (`self.SideWalkMeshes`)))
  (bind _outitem_2 (`KismetArrayLibrary.Array_Random` (`self.StreetMeshes`)))
  (if (`self.DoNotSpawnObstacle`)
    (if (== (`KismetMathLibrary.RandomIntegerInRange` 0 1) 0)
      (`|ExecutionSequence`
        (:`then_0`
          ;[0.1198 0.1198 0.1198] SideWalks - Obs 1 & 4
          (if (== (`KismetMathLibrary.RandomIntegerInRange` 0 1) 0)
            (`StaticMeshComponent.SetStaticMesh` (`self.Obstacle1`) _outitem)))
        (:`then_1`
          (if (== (`KismetMathLibrary.RandomIntegerInRange` 0 1) 0)
            (`StaticMeshComponent.SetStaticMesh` (`self.Obstacle4`) _outitem)))
        (:`then_2`
          ;[0.08333 0.08333 0.08333] Roads - Obs 2 & 3
          (if (`self.SpawnLane2Car`)
            (if (== (`KismetMathLibrary.RandomIntegerInRange` 0 2) 0)
              (`StaticMeshComponent.SetStaticMesh` (`self.Obstacle2`) _outitem_2))))
        (:`then_3`
          (if (`self.SpawnLane3Car`)
            (if (== (`KismetMathLibrary.RandomIntegerInRange` 0 2) 0)
              (`StaticMeshComponent.SetStaticMesh` (`self.Obstacle3`) _outitem_2))))))))

(fn `SpawnBuildings`
  (`StaticMeshComponent.SetStaticMesh` (`self.BuildingLeft`) (`KismetArrayLibrary.Array_Random` (`self.BuildingMeshes`)))
  (`StaticMeshComponent.SetStaticMesh` (`self.BuildingRight`) (`KismetArrayLibrary.Array_Random` (`self.BuildingMeshes`))))

(fn `SpawnCoins`
  (bind _returnvalue (select `int` (`self.CoinLane`) :`0` (`self.Obstacle1`) :`1` (`self.Obstacle2`) :`2` (`self.Obstacle3`) :`3` (`self.Obstacle4`)))
  (set `self.CoinLane` (`KismetMathLibrary.RandomIntegerInRange` 0 3))
  (`/Engine/EditorBlueprintResources/StandardMacros.IsValid` (`StaticMeshComponent.StaticMesh` _returnvalue)
    (:`Is Not Valid`
      (`|SpawnActorFromClass` "/Game/Blueprints/BP_Coin.BP_Coin_C" (`KismetMathLibrary.MakeTransform` (`SceneComponent.K2_GetComponentLocation` _returnvalue)) "Undefined" "MultiplyWithRoot" null null))))

(fn `UserConstructionScript`)